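; Main menu game mode for Tale that shows the menu and launches play as either a new or an existing game.
; ShowMainMenu creates and displays WBP_MainMenu and starts the background music; BeginPlay is empty, so it relies on an outside call.
; OnPlay stops the music, waits out a click sound, removes the menu, stores IsNewGame in the game instance and opens the configured level.
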(event Custom|OnPlay
  (params (IsNewGame :type Boolean))
  (bind _uibuttonnewsc (Variables|Default|GetUIButtonNewSC))
  (Audio|Components|Audio|Stop (Variables|Default|GetBackgroundMusicAudioComponent))
  (Audio|PlaySound2D _uibuttonnewsc 1.0 1.0 0.0 0 0)
  (Utilities|FlowControl|Delay (Variables|/Script/Engine.SoundBase|GetDuration _uibuttonnewsc))
  (Widget|RemovefromParent (Variables|Default|GetMainMenuWBPRef))
  (bind _asbp_tale_game_instance (Utilities|Casting|CastToBP_TaleGameInstance (Game|GetGameInstance)))
  (Variables|/Game/Tale/BP/BP_TaleGameInstance.BP_TaleGameInstance_C|SetIsNewGame _asbp_tale_game_instance IsNewGame)
  (Game|OpenLevel(byName) (Variables|Default|GetLevelName)))

(event EventBeginPlay)

(event EventTick
  (params (DeltaSeconds :type Float%20%28single-precision%29)))

(fn ConstructionScript)

(fn ShowMainMenu
  (bind _returnvalue (UserInterface|CreateWidget "/Game/Tale/UI/WBP_MainMenu.WBP_MainMenu_C"))
  (bind _output_get (Variables|Default|SetMainMenuWBPRef _returnvalue))
  (UserInterface|Viewport|AddtoViewport _output_get 0)
  (Audio|Components|Audio|Play (Variables|Default|GetBackgroundMusicAudioComponent) 0.0)
  (return))