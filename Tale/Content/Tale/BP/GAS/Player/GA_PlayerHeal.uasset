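; Gameplay ability that lets the player heal by consuming a health potion from the inventory.
; On activation it asks the player's inventory component for a potion, ending immediately if none is valid.
; Otherwise it triggers the character's Niagara effect and a sound, then applies GE_PlayerRecoverHealth to itself with a SetByCaller duration magnitude.
; It then removes the potion and ends without waiting for the effect.
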(event Ability|EventActivateAbility
  (bind _asbp_tale_player_character (Utilities|Casting|CastToBP_TalePlayerCharacter (Game|GetPlayerCharacter 0)))
  (bind (_player_inventory_item _isvalid) (Default|GetHealthPotion (Variables|/Game/Tale/BP/Player/BP_TalePlayerCharacter.BP_TalePlayerCharacter_C|GetBP_PlayerInventoryComponent _asbp_tale_player_character)))
  (if _isvalid
    (Components|Activation|Activate (Variables|/Game/Tale/BP/Player/BP_TalePlayerCharacter.BP_TalePlayerCharacter_C|GetNiagara _asbp_tale_player_character) false)
    (Audio|PlaySoundatLocation "/Game/Tale/Audio/SFX/healpop-46004.healpop-46004" (Transformation|GetActorLocation _asbp_tale_player_character) "0, 0, 0" 1.0 1.0 0.0 0 0 0 0)
    (bind _returnvalue (Ability|GameplayEffect|AssignTagSetbyCallerMagnitude (Ability|MakeOutgoingGameplayEffectSpec "/Game/Tale/BP/GAS/Player/GE_PlayerRecoverHealth.GE_PlayerRecoverHealth_C") "(TagName=\"Gameplay.Magnitude.Duration\")" 3.0))
    (Ability|ApplyGameplayEffectSpecToOwner _returnvalue)
    (Default|RemoveItem (Variables|/Game/Tale/BP/Player/BP_TalePlayerCharacter.BP_TalePlayerCharacter_C|GetBP_PlayerInventoryComponent _asbp_tale_player_character) _player_inventory_item)
    (Ability|EndAbility)
    (else
      (Ability|EndAbility))))

(event Ability|EventOnEndAbility
  (params (bWasCancelled :type Boolean)))