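; Game mode for the main menu that shows the menu widget with background music and launches the game level.
; BeginPlay limits FPS, flags the game instance as coming from the menu, then creates WBP_MainMenu with UI-only input and a visible cursor.
; OnPlay stops the music, waits out the New or Continue button sound, stores IsNewGame in BP_TaleGameInstance, then opens the level by name.
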(event Custom|OnPlay
  (params (IsNewGame :type Boolean))
  (bind _uibuttonnewsc (Variables|Default|GetUIButtonNewSC))
  (bind _uibuttoncontinuesc (Variables|Default|GetUIButtonContinueSC))
  ;[0.15 0.15 0.15 0.5] OnPlay
  (Audio|Components|Audio|Stop (Variables|Default|GetBackgroundMusicAudioComponent))
  (if IsNewGame
    (Audio|PlaySound2D _uibuttonnewsc 1.0 1.0 0.0 0 0)
    (Utilities|FlowControl|Delay (Variables|/Script/Engine.SoundBase|GetDuration _uibuttonnewsc))
    (else
      (Audio|PlaySound2D _uibuttoncontinuesc 1.0 1.0 0.0 0 0)
      (Utilities|FlowControl|Delay (Variables|/Script/Engine.SoundBase|GetDuration _uibuttoncontinuesc))))
  (bind _asbp_tale_game_instance (Utilities|Casting|CastToBP_TaleGameInstance (Game|GetGameInstance)))
  (Variables|/Game/Tale/BP/BP_TaleGameInstance.BP_TaleGameInstance_C|SetIsNewGame _asbp_tale_game_instance IsNewGame)
  (Game|OpenLevel(byName) (Variables|Default|GetLevelName)))

(event EventBeginPlay
  (Class|TaleGameModeBase|LimitFPS)
  (bind _asbp_tale_game_instance (Utilities|Casting|CastToBP_TaleGameInstance (Game|GetGameInstance)))
  (Variables|/Game/Tale/BP/BP_TaleGameInstance.BP_TaleGameInstance_C|SetIsFromMainMenu _asbp_tale_game_instance true)
  (CallFunction|ShowMainMenu))

(fn ConstructionScript)

(fn ShowMainMenu
  (bind _returnvalue (Game|GetPlayerController 0))
  (bind _returnvalue_2 (UserInterface|CreateWidget "/Game/Tale/UI/WBP_MainMenu.WBP_MainMenu_C" (Game|GetPlayerController 0)))
  (bind _output_get (Variables|Default|SetMainMenuWBPRef _returnvalue_2))
  (UserInterface|Viewport|AddtoViewport _output_get 0)
  (Audio|Components|Audio|Play (Variables|Default|GetBackgroundMusicAudioComponent) 0.0)
  (Input|EnableInput _returnvalue)
  (Input|SetInputModeUIOnly _returnvalue (Variables|Default|GetMainMenuWBPRef) "DoNotLock" false)
  (Variables|/Script/Engine.PlayerController|SetbShowMouseCursor _returnvalue true)
  (return))