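; Weapon pickup actor that represents a sword or shield inventory item placed in the world.
; The construction script switches on the item's Type, applying the item's mesh to WeaponMesh with a hand-set relative transform for each type.
; Its PickUp event only destroys the actor, with no overlap detection or inventory transfer in this graph.
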(event Custom|PickUp
  (Actor|DestroyActor))

(event EventBeginPlay)

(event Collision|EventActorBeginOverlap
  (params (OtherActor :type Actor%20Object%20Reference)))

(event EventTick
  (params (DeltaSeconds :type Float%20%28single-precision%29)))

(fn ConstructionScript
  (bind _weaponmesh (Variables|Default|GetWeaponMesh))
  (bind _weaponmesh_2 (Variables|Default|GetWeaponMesh))
  (bind _playerinventoryitem (Variables|Default|GetPlayerInventoryItem))
  (bind (_name _isstackable _quantity _thumbnail _type _mesh) (Utilities|Struct|BreakS_PlayerInventoryItem _playerinventoryitem))
  (switch Utilities|FlowControl|Switch|SwitchonE_ItemType _type
    (:NewEnumerator0
      (Components|StaticMesh|SetStaticMesh _weaponmesh _mesh)
      (Transformation|SetRelativeTransform _weaponmesh (Math|Transform|MakeTransform "-18.000000,0.000000,31.000000" "198.000000,0.000000,0.000000" "1.000000,1.000000,1.000000") false false))
    (:NewEnumerator2
      (Components|StaticMesh|SetStaticMesh _weaponmesh_2 _mesh)
      (Transformation|SetRelativeTransform _weaponmesh_2 (Math|Transform|MakeTransform "0, 0, 0" "0.000000,0.000000,20.000000" "1.000000,1.000000,1.000000") false false))))