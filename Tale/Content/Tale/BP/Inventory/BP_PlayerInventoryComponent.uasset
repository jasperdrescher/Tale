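; Player inventory component for the Tale character that stores picked-up items and drives a toggleable inventory widget.
; Interact takes the nearest overlapping weapon pickup, flags sword or shield ownership, then stacks onto a matching item or appends a new entry and reloads the widget.
; Number keys equip an owned sword or shield by setting its mesh on the right or left hand, with the sword also repositioning the weapon sphere.
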(event Custom|Reload%20Inventory
  ;[0.15 0.15 0.15 0.5] Reload Inventory
  (Default|LoadInventory (Variables|Default|GetPlayerInventoryWidgetRef) self))

(event Custom|TryEquipShield
  ;[0.15 0.15 0.15 0.5] TryEquipShield
  (if (Variables|Default|GetbHasShield)
    (bind _array_element (Utilities|Array|ForEachLoopwithBreak (Variables|Default|GetItems) :!label _label)
      (:LoopBody
        (switch Utilities|FlowControl|Switch|SwitchonE_ItemType (.Type (Utilities|Struct|BreakS_PlayerInventoryItem _array_element))
          (:NewEnumerator2
            (bind _returnvalue (Components|StaticMesh|SetStaticMesh (Variables|/Game/Tale/BP/Player/BP_TalePlayerCharacter.BP_TalePlayerCharacter_C|GetWeaponL (Variables|Default|GetPlayerCharacterRef)) (.Mesh (Utilities|Struct|BreakS_PlayerInventoryItem _array_element))))
            (if _returnvalue
              (goto _label Break))))))))

(event Custom|TryEquipSword
  (bind _playercharacterref (Variables|Default|GetPlayerCharacterRef))
  ;[0.15 0.15 0.15 0.5] TryEquipSword
  (if (Variables|Default|GetbHasSword)
    (bind _array_element (Utilities|Array|ForEachLoopwithBreak (Variables|Default|GetItems) :!label _label)
      (:LoopBody
        (switch Utilities|FlowControl|Switch|SwitchonE_ItemType (.Type (Utilities|Struct|BreakS_PlayerInventoryItem _array_element))
          (:NewEnumerator0
            (bind _returnvalue (Components|StaticMesh|SetStaticMesh (Variables|/Game/Tale/BP/Player/BP_TalePlayerCharacter.BP_TalePlayerCharacter_C|GetWeaponR _playercharacterref) (.Mesh (Utilities|Struct|BreakS_PlayerInventoryItem _array_element))))
            (if _returnvalue
              (Transformation|SetRelativeLocation (Variables|/Game/Tale/BP/Player/BP_TalePlayerCharacter.BP_TalePlayerCharacter_C|GetWeaponSphere _playercharacterref) "-1.690000,1.170000,110.690000" false false)
              (goto _label Break))))))))

(event Input|EnhancedActionEvents|EnhancedInputActionIA_Interact
  (params (ActionValue :type Boolean) (ElapsedSeconds :type Float%20%28double-precision%29) (TriggeredSeconds :type Float%20%28double-precision%29) (InputAction :type Input%20Action%20Object%20Reference :default "/Game/Tale/Input/Actions/IA_Interact.IA_Interact"))
  (bind _playercharacterref (Variables|Default|GetPlayerCharacterRef))
  ;[0.15 0.15 0.15 0.5] Pick up weapon
  (bind _asbp_weapon_pickup (Utilities|Casting|CastToBP_WeaponPickup (.ReturnValue (Actor|FindNearestActor (Transformation|GetWorldLocation (Variables|/Script/Engine.Character|GetMesh _playercharacterref)) (Collision|GetOverlappingActors _playercharacterref "/Game/Tale/BP/Inventory/BP_WeaponPickup.BP_WeaponPickup_C" :!class /Script/Engine.Actor)))))
  (Utilities|FlowControl|Sequence
    (:then_0
      (switch Utilities|FlowControl|Switch|SwitchonE_ItemType (.Type (Utilities|Struct|BreakS_PlayerInventoryItem (Variables|/Game/Tale/BP/Inventory/BP_WeaponPickup.BP_WeaponPickup_C|GetPlayerInventoryItem _asbp_weapon_pickup)))
        (:NewEnumerator0
          (Variables|Default|SetbHasSword true))
        (:NewEnumerator2
          (Variables|Default|SetbHasShield true))))
    (:then_1
      (bind _array_element (Utilities|Array|ForEachLoopwithBreak (Variables|Default|GetItems) :!label _label)
        (:LoopBody
          (if (< (.Quantity (Utilities|Struct|BreakS_PlayerInventoryItem _array_element)) 64)
            (if (and (Utilities|Enum|Equal(Enum) (.Name (Utilities|Struct|BreakS_PlayerInventoryItem (Variables|/Game/Tale/BP/Inventory/BP_WeaponPickup.BP_WeaponPickup_C|GetPlayerInventoryItem _asbp_weapon_pickup))) (.Name (Utilities|Struct|BreakS_PlayerInventoryItem _array_element))) (== (.IsStackable (Utilities|Struct|BreakS_PlayerInventoryItem (Variables|/Game/Tale/BP/Inventory/BP_WeaponPickup.BP_WeaponPickup_C|GetPlayerInventoryItem _asbp_weapon_pickup))) (.IsStackable (Utilities|Struct|BreakS_PlayerInventoryItem _array_element))))
              (Math|Integer|IncrementInt (.Quantity (Utilities|Struct|BreakS_PlayerInventoryItem _array_element))
                (:%20%20
                  (Audio|PlaySound2D "/Game/Tale/Audio/SFX/SC_ChimeNChomp.SC_ChimeNChomp" 1.0 1.0 0.0 0 0)
                  (Default|PickUp _asbp_weapon_pickup)
                  (goto _label Break))))))
        (:Completed
          (Utilities|IsValid _asbp_weapon_pickup
            (:Is%20Valid
              (Utilities|Array|Add (Variables|Default|GetItems) (Variables|/Game/Tale/BP/Inventory/BP_WeaponPickup.BP_WeaponPickup_C|GetPlayerInventoryItem _asbp_weapon_pickup))
              (Audio|PlaySound2D "/Game/Tale/Audio/SFX/SC_ChimeNChomp.SC_ChimeNChomp" 1.0 1.0 0.0 0 0)
              (Default|PickUp _asbp_weapon_pickup)
              (Default|LoadInventory (Variables|Default|GetPlayerInventoryWidgetRef) self))))))))

(event EventBeginPlay
  ;[0.2747 0.02843 0.02732] Begin Play
  (bind _asbp_tale_player_character (Utilities|Casting|CastToBP_TalePlayerCharacter (Components|GetOwner)))
  (Variables|Default|SetPlayerCharacterRef _asbp_tale_player_character)
  (bind _returnvalue (UserInterface|CreateWidget "/Game/Tale/UI/WBP_PlayerInventory.WBP_PlayerInventory_C"))
  (Variables|Default|SetPlayerInventoryWidgetRef _returnvalue)
  (Utilities|Array|Resize (Variables|Default|GetItems) 10)
  (CallFunction|ReloadInventory))

(event EventTick
  (params (DeltaSeconds :type Float%20%28single-precision%29)))

(event Input|KeyboardEvents|1
  (params (Key :type Key%20Structure :default "None"))
  (:Pressed
    (CallFunction|TryEquipSword)))

(event Input|KeyboardEvents|I
  (params (Key :type Key%20Structure :default "None"))
  (bind _playerinventorywidgetref (Variables|Default|GetPlayerInventoryWidgetRef))
  ;[0.15 0.15 0.15 0.5] Toggle inventory
  (:Pressed
    (if (Widget|IsVisible (Variables|Default|GetPlayerInventoryWidgetRef))
      (Widget|RemovefromParent _playerinventorywidgetref)
      (else
        (UserInterface|Viewport|AddtoViewport _playerinventorywidgetref 0)))))

(event Input|KeyboardEvents|2
  (params (Key :type Key%20Structure :default "None"))
  (:Pressed
    (CallFunction|TryEquipShield)))