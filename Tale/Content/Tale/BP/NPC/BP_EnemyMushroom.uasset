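; Mushroom enemy NPC that wakes up and turns to face the player while it can see them.
; PawnSensing flags sightings of Player-tagged pawns, and a timer matching the sensing interval clears the flag unless another sighting renews it.
; Each Tick copies that flag into the awake state, passes it to ABP_Mushroom and, while awake, snaps the actor's full rotation toward player pawn 0.
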(event OnSeePawn(PawnSensing)
  (params (Pawn :type Pawn%20Object%20Reference))
  (if (Actor|ActorHasTag Pawn "Player")
    (Variables|Default|SetHasSeenPlayer true)
    (Utilities|Time|SetTimerbyEvent (delegate Custom|ResetHasSeenPlayer) (Variables|/Script/AIModule.PawnSensingComponent|GetSensingInterval (Variables|Default|GetPawnSensing)))))

(event Custom|ResetHasSeenPlayer
  (Variables|Default|SetHasSeenPlayer false))

(event EventBeginPlay
  (|CallParentFunction))

(event Collision|EventActorBeginOverlap
  (params (OtherActor :type Actor%20Object%20Reference))
  (|CallParentFunction OtherActor) ; This node is disabled and will not be called.\nDrag off pins to build functionality.
)

(event EventTick
  (params (DeltaSeconds :type Float%20%28single-precision%29))
  (|CallParentFunction DeltaSeconds)
  (Utilities|FlowControl|Sequence
    (:then_0
      (if (Variables|Default|GetHasSeenPlayer)
        (Variables|Default|SetIsAwake true)
        (bind _asabp_mushroom (Utilities|Casting|CastToABP_Mushroom (Components|SkeletalMesh|GetAnimInstance (Variables|Character|GetMesh))))
        (Default|UpdateIsAwake _asabp_mushroom (Variables|Default|GetIsAwake))
        (else
          (Variables|Default|SetIsAwake false)
          (bind _asabp_mushroom_2 (Utilities|Casting|CastToABP_Mushroom (Components|SkeletalMesh|GetAnimInstance (Variables|Character|GetMesh))))
          (Default|UpdateIsAwake _asabp_mushroom_2 (Variables|Default|GetIsAwake)))))
    (:then_1
      (if (Variables|Default|GetIsAwake)
        (Transformation|SetActorRotation (Math|Rotator|FindLookatRotation (Transformation|GetActorLocation) (Transformation|GetActorLocation (Game|Player|GetPlayerPawn 0))))))))

(fn ConstructionScript
  (|CallParentFunction))