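; Slime enemy NPC that feeds perception state to its AI blackboard and keeps its attribute widget turned toward the camera.
; Pawn sensing flags that the player has been seen, while an attack-radius overlap stores the player and toggles the in-range flag.
; Damage and Attack events are empty; health, hit/death montage and random-section attack logic remains in the graph but is disconnected.
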(event OnComponentBeginOverlap(AttackRadius)
  (params (OverlappedComponent :type Primitive%20Component%20Object%20Reference) (OtherActor :type Actor%20Object%20Reference) (OtherComp :type Primitive%20Component%20Object%20Reference) (OtherBodyIndex :type Integer) (bFromSweep :type Boolean) (SweepResult :type Hit%20Result%20Structure%20%28by%20ref%29))
  ;[0.15 0.15 0.15 0.5] Attack radius
  (bind _asbp_tale_player_character (Utilities|Casting|CastToBP_TalePlayerCharacter OtherActor))
  (Variables|Default|SetPlayerRef _asbp_tale_player_character)
  (AI|Components|Blackboard|SetValueasBool (AI|GetBlackboard 0) (Utilities|Name|MakeLiteralName "IsInRangeOfPlayer") true))

(event OnComponentEndOverlap(AttackRadius)
  (params (OverlappedComponent :type Primitive%20Component%20Object%20Reference) (OtherActor :type Actor%20Object%20Reference) (OtherComp :type Primitive%20Component%20Object%20Reference) (OtherBodyIndex :type Integer))
  ;[0.15 0.15 0.15 0.5] Attack radius
  (Utilities|Casting|CastToBP_TalePlayerCharacter OtherActor)
  (AI|Components|Blackboard|SetValueasBool (AI|GetBlackboard 0) (Utilities|Name|MakeLiteralName "IsInRangeOfPlayer") false))

(event OnSeePawn(PawnSensing)
  (params (Pawn :type Pawn%20Object%20Reference))
  ;[0.15 0.15 0.15 0.5] Pawn sensing
  (Utilities|Casting|CastToBP_TalePlayerCharacter Pawn)
  (AI|Components|Blackboard|SetValueasBool (AI|GetBlackboard 0) (Utilities|Name|MakeLiteralName "HasSeenPlayer") true))

(event Custom|Attack
  ;[0.15 0.15 0.15 0.5] Attack
)

(event EventBeginPlay)

(event EventTick
  (params (DeltaSeconds :type Float%20%28single-precision%29))
  ;[0.15 0 0.01766 0.5] Event Tick
  (Transformation|SetWorldRotation (Variables|Default|GetEnemyAttributesWidgetComponent) (Math|Rotator|FindLookatRotation (Math|Conversions|ToVector(Float) (Class|GameplayStatics|GetWorldOriginLocation)) (Camera|GetCameraLocation (Game|GetPlayerCameraManager 0))) false false))

(event Game|Damage|EventAnyDamage
  (params (Damage :type Float%20%28single-precision%29) (DamageType :type Damage%20Type%20Object%20Reference) (InstigatedBy :type Controller%20Object%20Reference) (DamageCauser :type Actor%20Object%20Reference))
  ;[0.15 0.15 0.15 0.5] Any damage
)

(fn ConstructionScript)