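; BP_TaleGameInstance is the game instance that owns persistence of the player's health and position.
; On Init it loads the existing save slot, or creates a new BP_TaleSaveGame object in memory if none exists.
; Save writes both values into that cached object and saves it to the slot, while GetSaveGameData reads them back from the cache.
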(event Custom|Save
  (params (PlayerHealth :type Float%20%28double-precision%29) (PlayerPosition :type Transform))
  (bind _savegame (Variables|Default|GetSaveGame))
  ;[0.15 0.15 0.15 0.5] Save game
  (Variables|/Game/Tale/BP/BP_TaleSaveGame.BP_TaleSaveGame_C|SetPlayerHealth _savegame PlayerHealth)
  (Variables|/Game/Tale/BP/BP_TaleSaveGame.BP_TaleSaveGame_C|SetPlayerPosition _savegame PlayerPosition)
  (SaveGame|SaveGametoSlot _savegame (Variables|Default|GetSlot%20Name)))

(event Custom|Load
  (params (Slot%20name :type String))
  ;[0.15 0.15 0.15 0.5] Load game
  (bind _returnvalue (SaveGame|LoadGamefromSlot Slot%20name))
  (bind _asbp_tale_save_game (Utilities|Casting|CastToBP_TaleSaveGame _returnvalue))
  (Variables|Default|SetSaveGame _asbp_tale_save_game))

(event EventInit
  (bind _exists (CallFunction|HasSaveGame))
  (if _exists
    (CallFunction|Load (Variables|Default|GetSlot%20Name))
    (else
      (bind _returnvalue (SaveGame|CreateSaveGameObject "/Game/Tale/BP/BP_TaleSaveGame.BP_TaleSaveGame_C"))
      (Variables|Default|SetSaveGame _returnvalue))))

(fn GetSaveGameData
  (bind _savegame (Variables|Default|GetSaveGame))
  (return (Variables|/Game/Tale/BP/BP_TaleSaveGame.BP_TaleSaveGame_C|GetPlayerHealth _savegame) (Variables|/Game/Tale/BP/BP_TaleSaveGame.BP_TaleSaveGame_C|GetPlayerPosition _savegame)))

(fn HasSaveGame
  (bind _returnvalue (SaveGame|DoesSaveGameExist (Variables|Default|GetSlot%20Name)))
  (return _returnvalue))