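; Game mode for the Tale game that handles startup, saving and loading, pausing and the level-cleared screen.
; On BeginPlay it lifts the FPS limit, sets game-only input and loads saved data when continuing from the main menu.
; Save and load pass player health and position between the game instance and player character.
; Pause and level-clear events pause the game and show widgets with the cursor; pause also toggles back.
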(event Custom|SaveGame
  (bind _returnvalue (Game|GetPlayerCharacter 0))
  ;[0.15 0.15 0.15 0.5] Save game
  (bind _asbp_tale_game_instance (Utilities|Casting|CastToBP_TaleGameInstance (Game|GetGameInstance)))
  (bind _asbp_tale_player_character (Utilities|Casting|CastToBP_TalePlayerCharacter _returnvalue))
  (Default|Save _asbp_tale_game_instance (Variables|/Game/Tale/BP/Player/BP_TalePlayerCharacter.BP_TalePlayerCharacter_C|GetHealth _asbp_tale_player_character) (Transformation|GetActorTransform _returnvalue)))

(event Custom|LoadGame
  ;[0.15 0.15 0.15 0.5] Load game
  (bind _asbp_tale_player_character (Utilities|Casting|CastToBP_TalePlayerCharacter (Game|GetPlayerCharacter 0)))
  (bind _asbp_tale_game_instance (Utilities|Casting|CastToBP_TaleGameInstance (Game|GetGameInstance)))
  (bind (_playerhealth _playerposition) (Default|GetSaveGameData _asbp_tale_game_instance))
  (Default|OnLoadGame _asbp_tale_player_character _playerposition _playerhealth))

(event Custom|TogglePauseGame
  (bind _returnvalue (Game|GetPlayerController 0))
  (bind _returnvalue_2 (Game|GetPlayerController 0))
  ;[0.15 0.15 0.15 0.5] Toggle Pause Game
  (if (Game|IsGamePaused)
    (Widget|RemovefromParent (Variables|Default|GetPauseGameWidgetRef))
    (Game|SetGamePaused false)
    (Input|SetInputModeGameOnly _returnvalue_2 true)
    (Variables|/Script/Engine.PlayerController|SetbShowMouseCursor _returnvalue_2 false)
    (else
      (bind _returnvalue_3 (UserInterface|CreateWidget "/Game/Tale/UI/WBP_PauseMenu.WBP_PauseMenu_C" _returnvalue))
      (bind _output_get (Variables|Default|SetPauseGameWidgetRef _returnvalue_3))
      (UserInterface|Viewport|AddtoViewport _output_get 0)
      (Input|SetInputModeGameandUI _returnvalue _output_get "DoNotLock" true true)
      (Variables|/Script/Engine.PlayerController|SetbShowMouseCursor _returnvalue true)
      (Game|SetGamePaused true))))

(event EventBeginPlay
  ;[0.15 0 0.01539 0.5] BeginPlay
  (Class|TaleGameModeBase|RemoveFPSLimit)
  (Utilities|FlowControl|Sequence
    (:then_0
      (bind _asbp_tale_game_instance (Utilities|Casting|CastToBP_TaleGameInstance (Game|GetGameInstance)))
      (if (Variables|/Game/Tale/BP/BP_TaleGameInstance.BP_TaleGameInstance_C|GetIsFromMainMenu _asbp_tale_game_instance)
        (if (not (Variables|/Game/Tale/BP/BP_TaleGameInstance.BP_TaleGameInstance_C|GetIsNewGame _asbp_tale_game_instance))
          (CallFunction|LoadGame))))
    (:then_1
      (CallFunction|SetGameInput))))

(event EventLevelCleared
  (bind _returnvalue (Game|GetPlayerController 0))
  ;[0.15 0.15 0.15 0.5] Level Cleared
  (Audio|PlaySound2D "/Game/Tale/Audio/SFX/080245_sfx-magic-84935.080245_sfx-magic-84935" 1.0 1.0 0.0 0 0)
  (bind _returnvalue_2 (UserInterface|CreateWidget "/Game/Tale/UI/WBP_LevelCleared.WBP_LevelCleared_C" _returnvalue))
  (UserInterface|Viewport|AddtoViewport _returnvalue_2 0)
  (Input|SetInputModeGameandUI _returnvalue _returnvalue_2 "DoNotLock" true true)
  (Variables|/Script/Engine.PlayerController|SetbShowMouseCursor _returnvalue true)
  (Game|SetGamePaused true))

(fn ConstructionScript)

(fn SetGameInput
  (bind _returnvalue (Game|GetPlayerController 0))
  (Input|SetInputModeGameOnly _returnvalue false)
  (Variables|/Script/Engine.PlayerController|SetbShowMouseCursor _returnvalue false)
  (return))